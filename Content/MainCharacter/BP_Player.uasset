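; BP_Player is the player character Blueprint, handling movement, mouse look and switching between two cameras.
; Axis inputs move it along the capsule's forward and right vectors, with walk speed halved during full backward input.
; Look axes drive controller pitch and yaw.
; ChangeCamera flip-flops between MainCamera and ExtraCamera, enabling controller-yaw body rotation for ExtraCamera and disabling it for MainCamera.
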(event `InputAxis|MoveForwardBack`
  (params (AxisValue :type "Float (single-precision)"))
  (bind _charactermovement (`self.CharacterMovement`))
  ;[0.143 1 0.1146] Передвижение
  (`self.AddMovementInput` (`SceneComponent.GetForwardVector` (`self.CapsuleComponent`)) AxisValue)
  (set `CharacterMovementComponent.MaxWalkSpeed` 300.0 _charactermovement)
  (if (== AxisValue -1.0)
    (set `CharacterMovementComponent.MaxWalkSpeed` 150.0 _charactermovement)))

(event `InputAxis|MoveLeftRight`
  (params (AxisValue :type "Float (single-precision)"))
  ;[0.143 1 0.1146] Передвижение
  (`self.AddMovementInput` (`SceneComponent.GetRightVector` (`self.CapsuleComponent`)) AxisValue))

(event `InputAction|ChangeCamera`
  (params (Key :type "Key Structure"))
  ;[0.1303 0.3759 1] Пеключение камеры
  (:`Pressed`
    (`/Engine/EditorBlueprintResources/StandardMacros.FlipFlop`
      (:`A`
        (`ActorComponent.Deactivate` (`self.MainCamera`))
        (`ActorComponent.Activate` (`self.ExtraCamera`) false)
        (set `self.bUseControllerRotationYaw` true))
      (:`B`
        (`ActorComponent.Deactivate` (`self.ExtraCamera`))
        (`ActorComponent.Activate` (`self.MainCamera`) false)
        (set `self.bUseControllerRotationYaw` false)))))

(event `InputAxis|LookUpDown`
  (params (AxisValue :type "Float (single-precision)"))
  ;[1 0.4027 0.05604] Вращение мышкой
  (`self.AddControllerPitchInput` AxisValue))

(event `InputAxis|LookLeftRight`
  (params (AxisValue :type "Float (single-precision)"))
  ;[1 0.4027 0.05604] Вращение мышкой
  (`self.AddControllerYawInput` AxisValue))

(fn `UserConstructionScript`)